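; BP_NecroChef is an enemy Blueprint that plays a scripted sequence leading to the win level.
; On BeginPlay it waits, plays the Rules of Nature animation once on its mesh, then after a second delay opens WinLevel.
; The construction script only calls its parent, and a StopSound2D helper stops a valid audio component but is not called in these graphs.
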(event `self.ReceiveBeginPlay`
  (`KismetSystemLibrary.Delay` 5.0)
  (`SkeletalMeshComponent.SetAnimation` (`self.Mesh`) "/Game/MyContent/Animations/NecroChef/AS_Necrochef_RULES_OF_NATURE.AS_Necrochef_RULES_OF_NATURE")
  (`SkeletalMeshComponent.Play` (`self.Mesh`) false)
  (`KismetSystemLibrary.Delay` 4.0)
  (`GameplayStatics.OpenLevelBySoftObjectPtr` "/Game/MyContent/Levels/WinLevel.WinLevel"))

(fn `StopSound2D`
  (params (AudioComponent :type "AudioComponent Object Reference"))
  (`/Engine/EditorBlueprintResources/StandardMacros.IsValid` AudioComponent
    (:`Is Valid`
      (`AudioComponent.Stop` AudioComponent))
    (:`Is Not Valid`
      _))
  (return))

(fn `UserConstructionScript`
  (`parent.UserConstructionScript`))