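; Enemy actor that wanders between random targets, hurts the player on contact and can be killed by jumping on it.
; Capsule hits damage the enemy when the airborne player lands on top, otherwise the player if within collision distance.
; Damage is ignored during invincibility, which also swaps the mesh material; a one-second timer repicks AI move targets.
; Destruction updates the HUD kill count, spawning BP_NecroChef and clearing objective text from five kills onward.
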(event `self.CapsuleComponent.OnComponentHit`
  (params (HitComponent :type "PrimitiveComponent Object Reference") (OtherActor :type "Actor Object Reference") (OtherComp :type "PrimitiveComponent Object Reference") (NormalImpulse :type "Vector Structure") (Hit :type "HitResult Structure (by ref)"))
  ;[1 1 1] To fix BP_Projectile exception
  (`/Engine/EditorBlueprintResources/StandardMacros.IsValid` OtherActor
    (:`Is Valid`
      (if (`self.ActorHasTag` OtherActor "Player")
        (if (and (< (.z Hit_ImpactNormal) 0.0) (not (`NavMovementComponent.IsMovingOnGround` (`Character.CharacterMovement` (`GameplayStatics.GetPlayerCharacter` 0)))))
          (`GameplayStatics.ApplyDamage` self 100.0)
          (elif (<= (`KismetMathLibrary.VSize` (- (`self.K2_GetActorLocation` (`GameplayStatics.GetPlayerCharacter` 0)) (`self.K2_GetActorLocation`))) (`self.CollisionDistance`))
            (`GameplayStatics.ApplyDamage` (`GameplayStatics.GetPlayerCharacter` 0) 100.0)))))))

(event `self.ReceiveAnyDamage`
  (params (Damage :type "Float (single-precision)") (DamageType :type "DamageType Object Reference") (InstigatedBy :type "Controller Object Reference") (DamageCauser :type "Actor Object Reference"))
  (if (not (`self.IsInvincible?`))
    (bind _output_get (set `self.CurrentHealth` (`KismetMathLibrary.FClamp` (- (`self.CurrentHealth`) Damage) 0.0 (`self.MaxHealth`))))
    (if (<= _output_get 0.0)
      (`self.K2_DestroyActor`))))

(event `self.ReceiveDestroyed`
  (bind _hud (`self.GetHUD`))
  (bind _returnvalue_x (`KismetMathLibrary.BreakVector` (`self.K2_GetActorLocation` (`GameplayStatics.GetPlayerPawn` 0))))
  (`/Game/MyContent/Blueprints/HUD/WBP_HUD.UpdateKillCount` _hud)
  (if (>= (`/Game/MyContent/Blueprints/HUD/WBP_HUD.KillCount` _hud) 5)
    (`|SpawnActorFromClass` "/Game/MyContent/Blueprints/Enemies/BP_NecroChef.BP_NecroChef_C" (`KismetMathLibrary.MakeTransform` (`KismetMathLibrary.MakeVector` _returnvalue_x 1970.0 167.200099) (struct :`Yaw` 90.0)) "Undefined" "OverrideRootScale" null null)
    (`TextBlock.SetText` (`/Game/MyContent/Blueprints/HUD/WBP_HUD.TXT_ObjectiveInfo` (`self.GetHUD`)) "")))

(event `MoveEnemyToTargets`
  (`self.MoveEnemyToTarget` (`KismetArrayLibrary.Array_Random` (`self.Targets`)))
  (`KismetSystemLibrary.K2_SetTimer` null "MoveEnemyToTargets" 1.0))

(fn `DisableInvincibility`
  (set `self.IsInvincible?` false)
  (bind _mesh (`self.Mesh`)
    (:`then`
      (`PrimitiveComponent.SetMaterial` _mesh 0 (`self.M_NotInvincible`)))
    (:`else`)))

(fn `EnableInvincibility`
  (set `self.IsInvincible?` true)
  (bind _mesh (`self.Mesh`)
    (:`then`
      (`PrimitiveComponent.SetMaterial` _mesh 0 (`self.M_Invincible`)))
    (:`else`)))

(fn `GetHUD`
  (returns (HUD :type "/Game/MyContent/Blueprints/HUD/WBP_HUD Object Reference"))
  (bind _asbp_potato (cast `/Game/MyContent/Blueprints/BP_Potato` (`GameplayStatics.GetPlayerCharacter` 0))
    (:`then`
      _)
    (:`CastFailed`
      (`KismetSystemLibrary.PrintString` "ThirdPersonCharacter cast failed")))
  (return (`/Game/MyContent/Blueprints/BP_Potato.GetWBP_HUD` _asbp_potato)))

(fn `UserConstructionScript`)