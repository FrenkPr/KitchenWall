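; AI controller for shooter enemies that runs BT_ShooterEnemy and feeds its blackboard from AI perception.
; Sensing the player sets line of sight, cancels any pending patrol reset and starts a looping timer that updates the in-shoot-range flag by distance.
; Otherwise, if the sensed BP_Potato is grounded, it stops range checks and schedules GoToPatrol after a delay, so jumping does not break targeting.
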(event `self.ReceivePossess`
  (params (PossessedPawn :type "Pawn Object Reference"))
  (`parent.ReceivePossess` PossessedPawn)
  (`self.RunBehaviorTree` "/Game/MyContent/Blueprints/Enemies/AI/BehavoiurTrees/BT_ShooterEnemy.BT_ShooterEnemy"))

(event `CheckShootDistance`
  ;[1 1 1] Enemy can see player
  (if (<= (`KismetMathLibrary.VSize` (- (`self.K2_GetActorLocation` (`GameplayStatics.GetPlayerCharacter` 0)) (`self.K2_GetActorLocation` (`self.Possessed Pawn`)))) (`self.ShootingDistance`))
    (`BlackboardComponent.SetValueAsBool` (`self.Blackboard`) (`self.IsPlayerInShootRange`) true)
    (else
      (`BlackboardComponent.SetValueAsBool` (`self.Blackboard`) (`self.IsPlayerInShootRange`) false))))

(event `self.AIPerception.OnTargetPerceptionUpdated`
  (params (Actor :type "Actor Object Reference") (Stimulus :type "AIStimulus Structure"))
  ;[1 1 1] Checks if the player is in the
  ; enemy's sight
  (if (and (`self.ActorHasTag` Actor "Player") Stimulus_bSuccessfullySensed (`self.ActorHasTag` "ShooterEnemyCtrl"))
    ;[1 1 1] Enemy can see player
    (`KismetSystemLibrary.K2_ClearAndInvalidateTimerHandle` (`self.ResetBB_ValuesOnPatrolTimer`))
    (`BlackboardComponent.SetValueAsBool` (`self.Blackboard`) (`self.HasLineOfSight`) true)
    (bind _returnvalue (`KismetSystemLibrary.K2_SetTimerDelegate` (delegate `CheckShootDistance`) 0.1 true))
    (set `self.ShootPlayerTimer` _returnvalue)
    (else
      ;[1 1 1] Enemy can't see player
      ;;[1 1 1] Won't let the enemy lose the player as target while the player is jumping and is near to the enemy
      (bind _asthird_person_character (cast `/Game/MyContent/Blueprints/BP_Potato` Actor))
      (if (`NavMovementComponent.IsMovingOnGround` (`Character.CharacterMovement` _asthird_person_character))
        (bind _returnvalue_2 (`KismetSystemLibrary.K2_SetTimer` null "GoToPatrol" (`self.FromChaseToPatrolTime`)))
        (set `self.ResetBB_ValuesOnPatrolTimer` _returnvalue_2)
        (`KismetSystemLibrary.K2_ClearAndInvalidateTimerHandle` (`self.ShootPlayerTimer`))))))

(fn `UserConstructionScript`
  (`parent.UserConstructionScript`))