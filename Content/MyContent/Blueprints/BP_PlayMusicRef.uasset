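; BP_PlayMusicRef plays a music track as a 2D sound and tracks its playback position.
; BeginPlay spawns PlayMusic without auto-destroy and keeps the audio component in ACPlayMusic.
; While that component is playing, Tick adds world delta time to MusicTimeOffsetSecs, resetting it to zero at MusicDurationSecs.
; The position is an accumulated estimate; nothing here reads it back or restarts the sound.
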(event `self.ReceiveBeginPlay`
  (bind _returnvalue (`GameplayStatics.SpawnSound2D` "/Game/MyContent/Sounds/PlayMusic.PlayMusic" 1.0 1.0 0.0 null false false))
  (set `self.AC_PlayMusic` _returnvalue))

(event `self.ReceiveTick`
  (params (DeltaSeconds :type "Float (single-precision)"))
  (bind _ac_playmusic (`self.AC_PlayMusic`)
    (:`then`
      (if (`AudioComponent.IsPlaying` _ac_playmusic)
        (bind _output_get (set `self.MusicTimeOffsetSecs` (`KismetMathLibrary.FClamp` (+ (`self.MusicTimeOffsetSecs`) (`GameplayStatics.GetWorldDeltaSeconds`)) 0.0 (`self.MusicDurationSecs`))))
        (if (>= _output_get (`self.MusicDurationSecs`))
          (set `self.MusicTimeOffsetSecs` 0.0))))
    (:`else`)))

(fn `UserConstructionScript`)